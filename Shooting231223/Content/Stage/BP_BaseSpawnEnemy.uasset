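; BP_BaseSpawnEnemy is a stage wave actor that tracks its enemy ships and advances to the next stage when all are gone.
; On BeginPlay it fills AllEnemy from its Child Actor components that hold a BP_EnemyShip.
; Each Tick it prunes invalid entries by index while looping over the array.
; Once the array is empty, it spawns the NextStage class at the world origin and destroys itself.
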(event EventBeginPlay
  (for _array_element (Components|GetChildrenComponents (Variables|Default|GetDefaultSceneRoot) false)
    (bind _aschild_actor_component (Utilities|Casting|CastToChildActorComponent _array_element))
    (bind _asbp_enemy (Utilities|Casting|CastToBP_EnemyShip (Variables|/Script/Engine.ChildActorComponent|GetChildActor _aschild_actor_component)))
    (Utilities|Array|Add (Variables|Default|GetAllEnemy) _asbp_enemy)))

(event Collision|EventActorBeginOverlap
  (params (OtherActor :type Actor%20Object%20Reference)))

(event EventTick
  (params (DeltaSeconds :type Float%20%28single-precision%29))
  (bind _allenemy (Variables|Default|GetAllEnemy))
  (if (== (Utilities|Array|Length _allenemy) 0)
    (Game|SpawnActorfromClass (Variables|Default|GetNextStage) (Math|Transform|MakeTransform "0, 0, 0") "Undefined" 0 0)
    (Actor|DestroyActor)
    (else
      (for (_array_element _array_index) _allenemy
        (Utilities|IsValid _array_element
          (:Is%20Not%20Valid
            (Utilities|Array|RemoveIndex (Variables|Default|GetAllEnemy) _array_index)))))))

(fn ConstructionScript)