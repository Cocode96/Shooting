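; Player-fired projectile Blueprint that damages enemy ships.
; It plays a shot sound at its location on spawn, then moves each tick along its root's right vector at Speed, without sweep.
; On overlap with a BP_EnemyShip it calls that ship's TakeDamage with a fixed amount, spawns a BulletHit effect and destroys itself, ignoring other actors.
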(event EventBeginPlay
  (Audio|PlaySoundatLocation "/Game/resource/Shot.Shot" (Transformation|GetWorldLocation (Variables|Default|GetDefaultSceneRoot)) "0, 0, 0" 1.0 1.0 0.0 0 0 0 0))

(event Collision|EventActorBeginOverlap
  (params (OtherActor :type Actor%20Object%20Reference))
  (bind _asbp_enemy (Utilities|Casting|CastToBP_EnemyShip OtherActor))
  (Default|TakeDamage _asbp_enemy 4e+01)
  (Niagara|SpawnSystematLocation "/Game/fx/BulletHit.BulletHit" (Transformation|GetActorLocation))
  (Actor|DestroyActor self))

(event EventTick
  (params (DeltaSeconds :type Float%20%28single-precision%29))
  (Transformation|AddWorldOffset (Variables|Default|GetDefaultSceneRoot) (* (* DeltaSeconds (Variables|Default|GetSpeed)) (Math|Vector|GetRightVector (Variables|Default|GetDefaultSceneRoot))) false false))

(fn ConstructionScript)