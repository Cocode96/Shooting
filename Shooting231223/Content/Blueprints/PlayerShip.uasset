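; Player ship for a shooter, moving on the YZ plane from input axes and opening the NewWorld level on any actor overlap.
; Each tick, ClampShip keeps it on screen using bounds deprojected from the viewport size.
; Space toggles firing; Shoot re-arms its own timer and spawns PlayerBullets through PrimaryFire.
; LevelUp raises PlayerLevel, which adds up to two extra muzzles beside the main one.
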(event Custom|LevelUp
  (Math|Integer|IncrementInt (Variables|Default|GetPlayerLevel)))

(event Custom|Shoot
  ;[1 1 1] shoot ammo
  (Utilities|Time|SetTimerbyEvent (delegate Custom|Shoot) 0.2)
  (if (Variables|Default|GetIsShooting)
    (switch int (Variables|Default|GetPlayerLevel)
      (:Default
        (CallFunction|PrimaryFire (Variables|Default|GetCube3) :!label _label)
        (CallFunction|PrimaryFire (Variables|Default|GetCube2) :!label _label_2))
      (:0
        _)
      (:1
        (goto _label_2))
      (:2
        (goto _label)))
    (CallFunction|PrimaryFire (Variables|Default|GetScene))))

(event EventBeginPlay
  (Utilities|FlowControl|Delay 0.1)
  (Transformation|SetWorldTransform (Variables|Default|GetDefaultSceneRoot) (Math|Transform|MakeTransform "0.000000,-2000.000000,0.000000") false false)
  (CallFunction|Shoot))

(event Collision|EventActorBeginOverlap
  (params (OtherActor :type Actor%20Object%20Reference))
  (Game|OpenLevel(byName) "NewWorld"))

(event EventTick
  (params (DeltaSeconds :type Float%20%28single-precision%29))
  (bind _output_get (Variables|Default|SetDelta%20Location (* (Math|Vector|Normalize (Math|Vector|MakeVector 0.0 (Input|AxisValues|GetRight) (Input|AxisValues|GetUp))) (* (Variables|Default|GetSpeed) DeltaSeconds))))
  (Transformation|AddWorldOffset (Variables|Default|GetDefaultSceneRoot) _output_get false false)
  (CallFunction|ClampShip))

(event Input|AxisEvents|InputAxisUp
  (params (AxisValue :type Float%20%28single-precision%29)))

(event Input|KeyboardEvents|W
  (params (Key :type Key%20Structure :default "None"))
  ;[1 1 1] Move
)

(event Input|KeyboardEvents|SpaceBar
  (params (Key :type Key%20Structure :default "None"))
  (:Pressed
    (Variables|Default|SetIsShooting (!= (Variables|Default|GetIsShooting) true))))

(fn ConstructionScript)

(fn ClampShip
  (bind _returnvalue (Transformation|GetActorLocation))
  (bind _returnvalue_2 (Game|GetPlayerController 0))
  (bind _returnvalue_3 (Viewport|GetViewportSize))
  (bind (_x _y _z) (Class|KismetMathLibrary|BreakVector3f _returnvalue))
  (bind _worldposition (Class|GameplayStatics|DeprojectScreentoWorld _returnvalue_2 _returnvalue_3))
  (bind (_x_2 _y_2 _z_2) (Math|Vector|BreakVector _worldposition))
  (Transformation|SetWorldLocation (Variables|Default|GetDefaultSceneRoot) (Math|Vector|MakeVector _x (Math|Float|Clamp(Float) _y (* _y_2 -1.0) _y_2) (Math|Float|Clamp(Float) _z _z_2 (* _z_2 -1.0))) false false))

(fn PrimaryFire
  (params (Target :type Scene%20Component%20Object%20Reference))
  (bind _returnvalue (Transformation|GetWorldTransform Target))
  (bind (_location _rotation) (Math|Transform|BreakTransform _returnvalue))
  (Game|SpawnActorfromClass "/Game/Blueprints/PlayerBullet.PlayerBullet_C" (Math|Transform|MakeTransform _location _rotation) "Undefined" 0 0)
  (return))