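; BP_ShootingMode tracks the score for a shooting mode and shows it on screen.
; On BeginPlay it creates a BP_ScoreUI widget and adds it to the viewport.
; The ScoreUp event adds the given points to Score and pushes the new value to the widget as text.
; PlayerLevel derives the player's level from the score, scaled down by a fixed divisor.
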(event Custom|ScoreUp
  (params (point :type Integer))
  (bind _output_get (Variables|Default|SetScore (+ point (Variables|Default|GetScore))))
  (Default|SetScoreText (Variables|Default|GetScoreUI) (Utilities|Text|ToText(Integer) _output_get)))

(event EventBeginPlay
  (bind _returnvalue (UserInterface|CreateWidget "/Game/UI/BP_ScoreUI.BP_ScoreUI_C"))
  (bind _output_get (Variables|Default|SetScoreUI _returnvalue))
  (UserInterface|Viewport|AddtoViewport _output_get 0))

(event EventTick
  (params (DeltaSeconds :type Float%20%28single-precision%29)))

(fn ConstructionScript)

(fn PlayerLevel
  (return (/ (Variables|Default|GetScore) 10)))