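; Enemy ship for a shooting game that flies along negative Y, fires bullets and takes damage.
; A self-rescheduling timer, active while IsShooting is set, rotates the Scene component in steps and spawns EnemyBullet from it, producing a rotating spray.
; Zero HP spawns a destruction effect and calls ShipReset.
; ShipReset also runs past the Y limit, so both cases play an explosion, randomly drop an item, add score and destroy the ship.
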(event Custom|TakeDamage
  (params (Damage :type Float%20%28double-precision%29))
  (bind _output_get (Variables|Default|SetHP (- (Variables|Default|GetHP) Damage)))
  (if (<= _output_get 0.0)
    (Niagara|SpawnSystematLocation "/Game/fx/DestroyFx_1.DestroyFx_1" (Transformation|GetActorLocation) "0, 0, 0" "2.000000,2.000000,2.000000")
    (CallFunction|ShipReset)))

(event Custom|Shoot
  (if (Variables|Default|GetIsShooting)
    (Utilities|Time|SetTimerbyEvent (delegate Custom|Shoot) 0.1)
    (Transformation|AddRelativeRotation (Variables|Default|GetScene) "0, 0,10.000000" false false)
    (CallFunction|PrimaryFire (Variables|Default|GetScene))))

(event Custom|ItemSpawn
  (if (< (Math|Random|RandomInteger 100) 10)
    (Game|SpawnActorfromClass "/Game/Blueprints/Item.Item_C" (Math|Conversions|ToTransform(Vector) (Transformation|GetWorldLocation (Variables|Default|GetSphere))) "Undefined" 0 0)))

(event Custom|ShipReset
  (Audio|PlaySoundatLocation "/Game/resource/Explosion.Explosion" (Transformation|GetWorldLocation (Variables|Default|GetSphere)) "0, 0, 0" 1.0 1.0 0.0 0 0 0 0)
  (CallFunction|ItemSpawn)
  (bind _asbp_shooting_mode (Utilities|Casting|CastToBP_ShootingMode (Game|GetGameMode)))
  (Default|ScoreUp _asbp_shooting_mode 1)
  (Actor|DestroyActor))

(event EventBeginPlay
  (CallFunction|Shoot))

(event Collision|EventActorBeginOverlap
  (params (OtherActor :type Actor%20Object%20Reference)))

(event EventTick
  (params (DeltaSeconds :type Float%20%28single-precision%29))
  (bind _rootcomponent (Variables|Transformation|GetRootComponent))
  (Transformation|AddWorldOffset _rootcomponent (Math|Vector|MakeVector 0.0 (* (* DeltaSeconds (Variables|Default|GetSpeed)) -1.0) 0.0) false false)
  (if (< (.Y (Math|Vector|BreakVector (Transformation|GetWorldLocation _rootcomponent))) -3e+03)
    (CallFunction|ShipReset)))

(event Game|Damage|EventAnyDamage
  (params (Damage :type Float%20%28single-precision%29) (DamageType :type Damage%20Type%20Object%20Reference) (InstigatedBy :type Controller%20Object%20Reference) (DamageCauser :type Actor%20Object%20Reference))
  (CallFunction|TakeDamage Damage))

(fn ConstructionScript)

(fn PrimaryFire
  (params (Target :type Scene%20Component%20Object%20Reference))
  (bind _returnvalue (Transformation|GetWorldTransform Target))
  (bind (_location _rotation) (Math|Transform|BreakTransform _returnvalue))
  (Game|SpawnActorfromClass "/Game/Blueprints/EnemyBullet.EnemyBullet_C" (Math|Transform|MakeTransform _location _rotation) "Undefined" 0 0)
  (return))