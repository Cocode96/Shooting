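; Item is a pickup that homes in on the player's ship and levels it up when collected.
; On BeginPlay it caches the controlled PlayerShip, then each Tick moves straight toward it at Speed, without sweeping.
; Collection uses a per-frame distance check rather than overlap events: within a short radius it spawns a Niagara effect, destroys itself and calls LevelUp on the ship.
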(event EventBeginPlay
  (bind _asplayer_ship (Utilities|Casting|CastToPlayerShip (Pawn|GetControlledPawn (Game|GetPlayerController 0))))
  (Variables|Default|SetAs%20Player%20Ship _asplayer_ship))

(event Collision|EventActorBeginOverlap
  (params (OtherActor :type Actor%20Object%20Reference)))

(event EventTick
  (params (DeltaSeconds :type Float%20%28single-precision%29))
  (bind _as_player_ship (Variables|Default|GetAs%20Player%20Ship))
  (bind _defaultsceneroot (Variables|Default|GetDefaultSceneRoot))
  (bind _returnvalue (Transformation|GetWorldLocation _defaultsceneroot))
  (bind _rootcomponent (Variables|/Script/Engine.Actor|GetRootComponent _as_player_ship))
  (bind _returnvalue_2 (Transformation|GetWorldLocation _rootcomponent))
  (bind _returnvalue_3 (- _returnvalue_2 _returnvalue))
  (if (< (Math|Vector|VectorLength _returnvalue_3) 2e+02)
    (Niagara|SpawnSystematLocation "/Game/fx/DestroyFx_1.DestroyFx_1" (Transformation|GetActorLocation) "0, 0, 0" "2.000000,2.000000,2.000000")
    (Actor|DestroyActor)
    (Default|LevelUp (Variables|Default|GetAs%20Player%20Ship))
    (else
      (Transformation|AddWorldOffset (Variables|Default|GetDefaultSceneRoot) (* (Math|Vector|Normalize _returnvalue_3) (* DeltaSeconds (Variables|Default|GetSpeed))) false false))))

(fn ConstructionScript)